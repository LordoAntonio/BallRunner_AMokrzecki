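; BP_Goal is the level's finish trigger, with a Marcus component that spins a fixed step every tick.
; When the player pawn overlaps its Box, it starts a camera fade, prints a joking Polish win message and plays Ducky_sounds.
; It then reopens the current level by name, with no delay for the fade, and destroys itself.
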(event `self.ReceiveTick`
  (params (DeltaSeconds :type "Float (single-precision)"))
  (`SceneComponent.K2_AddLocalRotation` (`self.Marcus`) (struct :`Yaw` 2.0) false false))

(event `self.Box.OnComponentBeginOverlap`
  (params (OverlappedComponent :type "PrimitiveComponent Object Reference") (OtherActor :type "Actor Object Reference") (OtherComp :type "PrimitiveComponent Object Reference") (OtherBodyIndex :type Integer) (bFromSweep :type Boolean) (SweepResult :type "HitResult Structure (by ref)"))
  (if (== OtherActor (`GameplayStatics.GetPlayerPawn` 0))
    (`PlayerCameraManager.StartCameraFade` :`self` (`GameplayStatics.GetPlayerCameraManager` 0) :`FromAlpha` 0.0 :`ToAlpha` 1.0 :`Duration` 5.0)
    (`KismetSystemLibrary.PrintString` "Brawo! wygrałes nic :D mozesz zagrac jeszcze raz" true true (struct :`R` 1.0 :`G` 0.788641 :`B` 0.042006 :`A` 1.0) 5.0)
    (`GameplayStatics.PlaySound2D` "/Game/Imported/ducky_sounds.ducky_sounds" 1.0 1.0 0.0 null null)
    (`|ExecutionSequence`
      (:`then_0`
        (bind _returnvalue (`GameplayStatics.GetCurrentLevelName` true))
        (`GameplayStatics.OpenLevel` (`KismetStringLibrary.Conv_StringToName` _returnvalue)))
      (:`then_1`
        (`self.K2_DestroyActor`)))))

(fn `UserConstructionScript`)