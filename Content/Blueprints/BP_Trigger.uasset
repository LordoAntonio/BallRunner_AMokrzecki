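; BP_Trigger is a fall-out kill volume that restarts the current level when the player enters it.
; A per-frame MoveComponentTo/Delay loop keeps it under the player in X and Y at fixed height, so one actor covers the whole scene.
; Overlap fades out, plays a game-over sound, increments Retry in the BP_retry_counter GameInstance, then reloads the level.
; BeginPlay also fades in, starts music and prints the attempt count.
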(event `self.Box.OnComponentBeginOverlap`
  (params (OverlappedComponent :type "PrimitiveComponent Object Reference") (OtherActor :type "Actor Object Reference") (OtherComp :type "PrimitiveComponent Object Reference") (OtherBodyIndex :type Integer) (bFromSweep :type Boolean) (SweepResult :type "HitResult Structure (by ref)"))
  (if (== OtherActor (`GameplayStatics.GetPlayerPawn` 0))
    (bind _returnvalue (`GameplayStatics.GetCurrentLevelName` true))
    (`PlayerCameraManager.StartCameraFade` :`self` (`GameplayStatics.GetPlayerCameraManager` 0) :`FromAlpha` 0.0 :`ToAlpha` 2.0 :`Duration` 1.0)
    (`GameplayStatics.PlaySound2D` "/Game/Imported/game_over.game_over" 1.0 1.0 0.0 null null)
    (`KismetSystemLibrary.Delay` (- 1.0 0.2))
    (bind _asbp_retry_counter (cast `/Game/Blueprints/BP_retry_counter` (`GameplayStatics.GetGameInstance`)))
    (set `/Game/Blueprints/BP_retry_counter.retry` (+ (`/Game/Blueprints/BP_retry_counter.retry` _asbp_retry_counter) 1) _asbp_retry_counter)
    (`GameplayStatics.OpenLevel` (`KismetStringLibrary.Conv_StringToName` _returnvalue))))

(event `self.ReceiveBeginPlay`
  (bind _defaultsceneroot (`self.DefaultSceneRoot`))
  (bind (_returnvalue_x _returnvalue_y) (`KismetMathLibrary.BreakVector` (`self.K2_GetActorLocation` (`GameplayStatics.GetPlayerPawn` 0))))
  (bind (_returnvalue_x_2 _returnvalue_y_2 _returnvalue_z) (`KismetMathLibrary.BreakVector` (`SceneComponent.K2_GetComponentLocation` _defaultsceneroot)))
  (`|ExecutionSequence`
    (:`then_0`
      (`PlayerCameraManager.StartCameraFade` :`self` (`GameplayStatics.GetPlayerCameraManager` 0) :`FromAlpha` 1.0 :`Duration` 1.0))
    (:`then_1`
      ;[1 1 1] Zrobiłem takie cos, zeby ta kolizja sledzila gracza i dzieki temu potrzebny jest tylko jeden aktor na cala scene, wystarczy zeby kulka smutno zaczela spadac w ciemna przestrzen :)
      (`KismetSystemLibrary.MoveComponentTo` _defaultsceneroot (`KismetMathLibrary.MakeVector` _returnvalue_x _returnvalue_y _returnvalue_z) (struct) false false 0.0 :!label _label)
      (`KismetSystemLibrary.Delay` 0.0)
      (goto _label))
    (:`then_2`
      (`GameplayStatics.PlaySound2D` "/Game/Imported/song_vaporwave.song_vaporwave" 0.4 0.9 0.0 null null))
    (:`then_3`
      (bind _asbp_retry_counter (cast `/Game/Blueprints/BP_retry_counter` (`GameplayStatics.GetGameInstance`)))
      (`KismetSystemLibrary.PrintString` (`KismetStringLibrary.Concat_StrStr` "Wlasnie tracisz czas na " (`KismetStringLibrary.Conv_IntToString` (`/Game/Blueprints/BP_retry_counter.retry` _asbp_retry_counter)) " podejscie ") true true (struct :`R` 1.0 :`G` 0.601165 :`B` 0.084162 :`A` 1.0) 5.0))))

(fn `UserConstructionScript`)